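; Actor that plays creepy ambient audio in a level when the game instance's Punish flag is set.
; On BeginPlay it checks that flag, starts the CreepyAudio component and subscribes to the game state's round stage change event.
; When the round reaches the Dice Roll stage, it fades the audio out over several seconds.
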(event `self.ReceiveBeginPlay`
  (bind _asbp_game_instance (cast `/Game/Blueprints/BP_GameInstance` (`GameplayStatics.GetGameInstance`)))
  (if (`/Game/Blueprints/BP_GameInstance.Punish` _asbp_game_instance)
    (`AudioComponent.Play` (`self.CreepyAudio`) 0.0)
    (bind _asbp_game_state (cast `/Game/Blueprints/BP_GameState` (`GameplayStatics.GetGameState`)))
    (add `/Game/Blueprints/BP_GameState.RoundStageChange` _asbp_game_state (delegate `OnRoundChange`))))

(event `OnRoundChange`
  (params (newStage :type "/Game/Blueprints/E_RoundStage Enum" :default "NewEnumerator0"))
  (switch `/Game/Blueprints/E_RoundStage` newStage
    (:`NewEnumerator3`
      (`AudioComponent.FadeOut` (`self.CreepyAudio`) 10.0 0.0 "Linear"))))

(fn `UserConstructionScript`)