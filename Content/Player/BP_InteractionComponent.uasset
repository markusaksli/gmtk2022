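; Player interaction component that detects interactable items in front of the first-person camera and triggers their use.
; Each Tick it line-traces along the camera's forward vector up to a max distance, caching any BPI_Interactable hit.
; It shows or hides the HUD interaction icon as that target changes, fetching the HUD from the game mode when needed.
; InteractWithItem forwards the player inventory to the cached target through the interface.
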(event `self.ReceiveBeginPlay`
  ;[1 1 1] Set camera ref
  (bind _asbp_first_person_character (cast `/Game/Player/BP_FirstPersonCharacter` (`self.GetOwner`)))
  (set `self.Camera` (`/Game/Player/BP_FirstPersonCharacter.FirstPersonCamera` _asbp_first_person_character)))

(event `self.ReceiveTick`
  (params (DeltaSeconds :type "Float (single-precision)"))
  (bind _camera (`self.Camera`))
  (bind _returnvalue (`SceneComponent.K2_GetComponentLocation` _camera))
  (bind _interactionicon (`/Game/HUD/WBP_HUD.InteractionIcon` (`self.WBP_HUDref`)))
  (bind _returnvalue_2 (`Widget.IsVisible` _interactionicon))
  ;[1 1 1] Item interaction line trace
  (`self.WBP_HUDref`
    (:`then`
      _)
    (:`else`
      ;;[1 1 1] Set HUD ref
      (bind _asbp_game_mode (cast `/Game/Blueprints/BP_GameMode` (`GameplayStatics.GetGameMode`)))
      (set `self.WBP_HUDref` (`/Game/Blueprints/BP_GameMode.WBP_HUDref` _asbp_game_mode))))
  (bind (_outhit _returnvalue_3) (`KismetSystemLibrary.LineTraceSingle` _returnvalue (+ _returnvalue (* (`SceneComponent.GetForwardVector` _camera) (`self.MaxInteractionDistance`))) "TraceTypeQuery1"))
  (if _returnvalue_3
    (bind (_bblockinghit _binitialoverlap _time _distance _location _impactpoint _normal _impactnormal _physmat _hitactor) (`GameplayStatics.BreakHitResult` _outhit))
    (cast `/Game/InteractableItems/Misc/BPI_Interactable` _hitactor
      (:`then`
        ;;[1 1 1] Set ref
        (bind _activeinteractableitemref (`self.ActiveInteractableItemRef`)
          (:`then`
            (if (!= _hitactor _activeinteractableitemref)
              (set `self.ActiveInteractableItemRef` _hitactor :!label _label)
              ;;[1 1 1] Set icon visible
              (if (not _returnvalue_2)
                (`Widget.SetVisibility` _interactionicon "Visible"))))
          (:`else`
            (goto _label))))
      (:`CastFailed`
        ;;[1 1 1] Clear ref
        (`self.ActiveInteractableItemRef` :!label _label_2
          (:`then`
            (set `self.ActiveInteractableItemRef` null)
            ;;[1 1 1] Set icon invisible
            (if _returnvalue_2
              (`Widget.SetVisibility` _interactionicon "Hidden")))
          (:`else`))))
    (else
      (goto _label_2))))

(event `InteractWithItem`
  (params (PlayerInventory :type "Set of /Game/InteractableItems/Misc/E_InventoryItem Enum"))
  ;[1 1 1] Trigger interaction
  (bind _activeinteractableitemref (`self.activeInteractableItemRef`)
    (:`then`
      (if (`KismetSystemLibrary.DoesImplementInterface` _activeinteractableitemref "/Game/InteractableItems/Misc/BPI_Interactable.BPI_Interactable_C")
        (bind _asbpi_interactable (cast `/Game/InteractableItems/Misc/BPI_Interactable` _activeinteractableitemref))
        (`/Game/InteractableItems/Misc/BPI_Interactable.InteractWithItem` _asbpi_interactable PlayerInventory)))
    (:`else`)))