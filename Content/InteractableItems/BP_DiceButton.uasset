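; BP_DiceButton is an interactable arrow button attached as a child actor to a BP_Dice, used to raise or lower that die's value.
; On BeginPlay it caches the parent dice and sets its text to ">" or "<" depending on the Add flag.
; Interacting calls Increment on the dice when enabled, and ToggleEnable switches that enabled state along with the text color.
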(event `/Game/InteractableItems/Misc/BI_Interactable.InteractWithItem`
  (params (PlayerInventory :type "Set of /Game/InteractableItems/Misc/E_InventoryItem Enum" :default _))
  (if (`self.enabled`)
    (`/Game/Blueprints/BP_Dice.Increment` (`self.dice`) (`self.add`))))

(event `self.ReceiveBeginPlay`
  (bind _asbp_dice (cast `/Game/Blueprints/BP_Dice` (`self.GetParentActor`)))
  (set `self.dice` _asbp_dice)
  (`TextRenderComponent.K2_SetText` (`self.TextRender`) (select `bool` (`self.add`) :`false` (`KismetTextLibrary.Conv_StringToText` "<") :`true` (`KismetTextLibrary.Conv_StringToText` ">"))))

(fn `ToggleEnable`
  (params (enable :type Boolean))
  (`TextRenderComponent.SetTextRenderColor` (`self.TextRender`) (select `bool` enable :`false` (`self.disabledColor`) :`true` (`self.enabledColor`)))
  (set `self.enabled` enable))

(fn `UserConstructionScript`)