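; BP_Interactable_2 is an interactable item that shows its interaction text as a HUD subtitle and adds itself to the inventory.
; On InteractwithItem it calls SetSubtitleText on the HUD widget, then AddItemToInventory on its BPAddToInventory member.
; The HUD reference is fetched lazily from BP_GameMode when it is null, then cached for reuse.
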(event `/Game/InteractableItems/BPI_Interactable.InteractWithItem`
  (if (not (!= (`self.WBP_HUDref`) null))
    ;[1 1 1] Set HUD ref if it's null
    (bind _asbp_game_mode (cast `/Game/Blueprints/BP_GameMode` (`GameplayStatics.GetGameMode`)))
    (set `self.WBP_HUDref` (`/Game/Blueprints/BP_GameMode.WBP_HUDref` _asbp_game_mode)))
  (`/Game/HUD/WBP_HUD.Set Subtitle Text` (`self.WBP_HUDref`) (`self.InteractionText`))
  (`/Game/InteractableItems/BP_AddToInventory.AddItemToInventory` (`self.BP_AddToInventory`)))

(fn `UserConstructionScript`)