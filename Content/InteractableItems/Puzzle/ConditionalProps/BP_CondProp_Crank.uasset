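; BP_CondProp_Crank is a conditional puzzle prop: a crank that removes the gate when the player has all necessary items.
; It extends the parent interaction, continuing it until it should finish, then hides the dialogue box and checks the items.
; On success it plays crank and water-door sounds, destroys the first "Gate"-tagged actor and itself.
; Movement is restored either way; on failure the dialogue state resets.
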(event `/Game/InteractableItems/Misc/BI_Interactable.InteractWithItem`
  (params (PlayerInventory :type "Set of /Game/InteractableItems/Misc/E_InventoryItem Enum" :default _))
  (`parent.InteractWithItem` PlayerInventory)
  ;[1 1 1] Should finish interacting?
  (if (`self.ShouldFinishInteracting?`)
    (`Widget.SetVisibility` (`/Game/HUD/WBP_HUD.DialogueTextBox` (`self.WBP_HUDref`)) "Hidden")
    (bind _hasallitems (`self.DoesPlayerHaveAllNecessaryItems`))
    (if _hasallitems
      (bind _outactors (`GameplayStatics.GetAllActorsWithTag` "Gate"))
      (`GameplayStatics.PlaySoundAtLocation` "/Game/Sounds/SFX/SFX_Wheel_Crank.SFX_Wheel_Crank" (`SceneComponent.K2_GetComponentLocation` (`self.Box`)) (struct) 1.0 1.0 0.0 "/Game/Sounds/SFX/SA_DiceATT.SA_DiceATT" null null null)
      (bind _output (`|GetArrayItem` _outactors))
      (`GameplayStatics.PlaySoundAtLocation` "/Game/Sounds/SFX/SFX_Door_Water.SFX_Door_Water" (`SceneComponent.K2_GetComponentLocation` (`Actor.RootComponent` _output)) (struct) 1.0 1.0 0.0 "/Game/Sounds/SFX/SA_DiceATT.SA_DiceATT" null null null)
      (`self.K2_DestroyActor` _output))
    (`/Game/InteractableItems/Misc/BC_DisableMovement.DisableMovement` (`self.BC_DisableMovement`) false)
    (if _hasallitems
      (`self.K2_DestroyActor`)
      (else
        (set `self.CurrentTextline` 0)
        (set `self.StartedInteracting` false)))
    (else
      (`self.KeepInteracting`))))

(fn `UserConstructionScript`)