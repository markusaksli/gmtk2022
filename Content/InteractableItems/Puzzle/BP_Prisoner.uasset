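; BP_Prisoner is an interactable puzzle NPC whose dialogue changes with the game round and eventually rewards the player with an item.
; SetInteractionTextlines picks lines from Round and HasInteractedWithPrisoner on the GameInstance, which BeginPlay resets in round 1.
; After round 1, an earlier talk plus all required items selects GiveCoinText.
; Finishing that dialogue, detected by array comparison, adds the item, plays a pickup sound and destroys the prisoner.
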(event `self.ReceiveBeginPlay`
  (bind _asbp_game_instance (cast `/Game/Blueprints/BP_GameInstance` (`GameplayStatics.GetGameInstance`) :!pure true))
  (if (== (`/Game/Blueprints/BP_GameInstance.Round` _asbp_game_instance) 1)
    (set `/Game/Blueprints/BP_GameInstance.hasInteractedWithPrisoner` false _asbp_game_instance)))

(event `/Game/InteractableItems/Misc/BI_Interactable.InteractWithItem`
  (params (PlayerInventory :type "Set of /Game/InteractableItems/Misc/E_InventoryItem Enum" :default _))
  (bind _returnvalue (`KismetArrayLibrary.Array_Identical` (`self.InteractionText`) (`self.GiveCoinText`)))
  (`parent.InteractWithItem` PlayerInventory)
  (if (not (`self.StartedInteracting`))
    (`self.SetInteractionTextlines`))
  ;[1 1 1] Should finish interacting?
  (if (`self.ShouldFinishInteracting?`)
    (`Widget.SetVisibility` (`/Game/HUD/WBP_HUD.DialogueTextBox` (`self.WBP_HUDref`)) "Hidden")
    (if _returnvalue
      (`/Game/InteractableItems/Misc/BC_AddToInventory.AddItemToInventory` (`self.BP_AddToInventory`))
      (`GameplayStatics.PlaySoundAtLocation` "/Game/Sounds/SFX/Iteam_PickUp/SC_ItemPickup.SC_ItemPickup" (`SceneComponent.K2_GetComponentLocation` (`self.Box_0`)) (struct) 1.0 1.0 0.0 "/Game/Sounds/SFX/SA_DiceATT.SA_DiceATT" null null null))
    (`/Game/InteractableItems/Misc/BC_DisableMovement.DisableMovement` (`self.BP_DisableMovement`) false)
    (if _returnvalue
      (`self.K2_DestroyActor`)
      (else
        (set `self.CurrentTextline` 0)
        (set `self.StartedInteracting` false)))
    (else
      (`self.KeepInteracting`))))

(fn `DoesPlayerHaveAllNecessaryItems`
  (returns (HasAllItems :type Boolean))
  (for _array_element (`self.ItemsToCheckFor`)
    (if (not (`BlueprintSetLibrary.Set_Contains` (`self.Player Inventory`) _array_element))
      (return false)))
  (return true))

(fn `SetInteractionTextlines`
  (locals (BP_GameInstanceRef :type "/Game/Blueprints/BP_GameInstance Object Reference"))
  (bind _asbp_game_instance (cast `/Game/Blueprints/BP_GameInstance` (`GameplayStatics.GetGameInstance`)))
  (bind _output_get (set `local.BP_GameInstanceRef` _asbp_game_instance))
  (if (> (`/Game/Blueprints/BP_GameInstance.Round` _output_get) 1)
    (bind _hasallitems (`self.DoesPlayerHaveAllNecessaryItems`))
    (if (and _hasallitems (`/Game/Blueprints/BP_GameInstance.hasInteractedWithPrisoner` (`local.BP_GameInstanceRef`)))
      (set `self.InteractionText` (`self.GiveCoinText`))
      (else
        (set `self.InteractionText` (`self.PostRound3Text`))
        (set `/Game/Blueprints/BP_GameInstance.hasInteractedWithPrisoner` true (`local.BP_GameInstanceRef`))))
    (elif (== (`/Game/Blueprints/BP_GameInstance.Round` (`local.BP_GameInstanceRef`)) 1)
      (set `self.InteractionText` (`self.Round2Text`))
      (elif (`/Game/Blueprints/BP_GameInstance.hasInteractedWithPrisoner` (`local.BP_GameInstanceRef`))
        (set `self.InteractionText` (`self.HasInteractedText`))
        (else
          (set `self.InteractionText` (`self.IntroText`))
          (set `/Game/Blueprints/BP_GameInstance.hasInteractedWithPrisoner` true (`local.BP_GameInstanceRef`)))))))

(fn `UserConstructionScript`)