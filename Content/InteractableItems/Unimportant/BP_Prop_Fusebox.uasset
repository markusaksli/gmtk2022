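; Interactable fusebox prop that shows a multi-line monologue, chosen by whether the player's inventory holds all required items.
; On first interaction it picks the text set, falling back to the has-items text if the missing-items text is empty.
; Each interaction finishes the line being typed or writes the next through the game mode's HUD widget.
; Movement and the interaction icon are disabled until the last line is dismissed.
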(event `/Game/InteractableItems/Misc/BPI_Interactable.InteractWithItem`
  (params (PlayerInventory :type "Set of /Game/InteractableItems/Misc/E_InventoryItem Enum" :default _))
  (bind _wbp_hudref (`self.WBP_HUDref`))
  (bind (_output_textline _output_charspersecond) (break `/Game/InteractableItems/Misc/S_TextLineInfo` (`|GetArrayItem` (`self.InteractionText`) (`self.CurrentTextline`))))
  (bind _interactionicon (`/Game/HUD/WBP_HUD.InteractionIcon` (`self.WBP_HUDref`)))
  (set `self.Player Inventory` PlayerInventory)
  (if (not (!= (`self.WBP_HUDref`) null))
    ;[1 1 1] Set HUD ref if it's null
    (bind _asbp_game_mode (cast `/Game/Blueprints/BP_GameMode` (`GameplayStatics.GetGameMode`)))
    (set `self.WBP_HUDref` (`/Game/Blueprints/BP_GameMode.WBP_HUDref` _asbp_game_mode)))
  (if (not (`self.StartedInteracting`))
    (`self.SetInteractionTextlines`))
  ;[1 1 1] Should finish interacting?
  (if (and (== (`self.CurrentTextline`) (`KismetArrayLibrary.Array_Length` (`self.InteractionText`))) (not (`/Game/HUD/WBP_HUD.IsWriting` (`self.WBP_HUDref`))))
    (`Widget.SetVisibility` (`/Game/HUD/WBP_HUD.TextBox` (`self.WBP_HUDref`)) "Hidden")
    (`/Game/InteractableItems/Misc/BP_DisableMovement.DisableMovement` (`self.BP_DisableMovement`) false)
    (`Widget.SetVisibility` _interactionicon "Visible")
    (set `self.CurrentTextline` 0)
    (set `self.StartedInteracting` false)
    (elif (`/Game/HUD/WBP_HUD.IsWriting` _wbp_hudref)
      (`/Game/HUD/WBP_HUD.FinishWritingCurrentLine` _wbp_hudref)
      (else
        (`/Game/HUD/WBP_HUD.WriteMonologue` (`self.WBP_HUDref`) _output_textline _output_charspersecond)
        (`/Engine/EditorBlueprintResources/StandardMacros.IncrementInt` (`self.CurrentTextline`)
          (:`  `
            (if (not (`self.StartedInteracting`))
              (`Widget.SetVisibility` (`/Game/HUD/WBP_HUD.TextBox` (`self.WBP_HUDref`)) "Visible")
              (`Widget.SetVisibility` _interactionicon "Hidden")
              (`/Game/InteractableItems/Misc/BP_DisableMovement.DisableMovement` (`self.BP_DisableMovement`) true)
              (if (not (`self.StartedInteracting`))
                (set `self.StartedInteracting` true)))))))))

(fn `DoesPlayerHaveAllNecessaryItems`
  (returns (HasAllItems :type Boolean))
  (for _array_element (`self.ItemsToCheckFor`)
    (if (not (`BlueprintSetLibrary.Set_Contains` (`self.Player Inventory`) _array_element))
      (return false)))
  (return true))

(fn `SetInteractionTextlines`
  (bind _hasallitems (`self.DoesPlayerHaveAllNecessaryItems`))
  (if (and (not _hasallitems) (`KismetArrayLibrary.Array_IsNotEmpty` (`self.DoesNotHaveAllItemsText`)))
    (set `self.InteractionText` (`self.DoesNotHaveAllItemsText`))
    (else
      (set `self.InteractionText` (`self.HasAllItemsText`)))))

(fn `UserConstructionScript`)