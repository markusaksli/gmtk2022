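; BP_Dice is an in-world dice prediction panel where a number from 0 to 6 is picked during the Dice Roll stage.
; It gathers child BP_DiceButton actors and follows BP_GameState round stage changes, enabling them at Dice Roll and disabling them with a roll sound at Round End.
; Increment steps the clamped prediction on the text display unless Rolling is set.
; The Roll event is an empty stub.
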(event `self.ReceiveBeginPlay`
  (for _array_element (`self.GetAllChildActors` true)
    (bind _asbp_dice_button (cast `/Game/InteractableItems/BP_DiceButton` _array_element))
    (`KismetArrayLibrary.Array_Add` (`self.buttons`) _asbp_dice_button))
  (`self.ToggleEnable` false)
  (bind _asbp_game_state (cast `/Game/Blueprints/BP_GameState` (`GameplayStatics.GetGameState`)))
  (add `/Game/Blueprints/BP_GameState.RoundStageChange` _asbp_game_state (delegate `OnRoundStageChange`)))

(event `OnRoundStageChange`
  (params (newStage :type "/Game/Blueprints/E_RoundStage Enum" :default "NewEnumerator0"))
  (switch `/Game/Blueprints/E_RoundStage` newStage
    (:`NewEnumerator3`
      (`self.ToggleEnable` true))
    (:`NewEnumerator4`
      (`self.ToggleEnable` false)
      (`GameplayStatics.PlaySoundAtLocation` "/Game/Sounds/SFX/SFX_Dice_Roll.SFX_Dice_Roll" (`SceneComponent.K2_GetComponentLocation` (`self.Display`)) (struct) 1.0 1.0 0.0 "/Game/Sounds/DefaultSoundAttenuation.DefaultSoundAttenuation" null null null))))

(event `Roll`)

(fn `Increment`
  (params (add :type Boolean))
  (if (not (`self.rolling`))
    (bind _output_get (set `self.prediction` (`KismetMathLibrary.Clamp` (+ (`self.prediction`) (select `bool` add :`false` -1 :`true` 1)) 0 6)))
    (`TextRenderComponent.K2_SetText` (`self.Display`) (`KismetTextLibrary.Conv_IntToText` _output_get))
    (`GameplayStatics.PlaySoundAtLocation` "/Game/Sounds/SFX/SFX_Button.SFX_Button" (`SceneComponent.K2_GetComponentLocation` (`self.Display`)) (struct) 1.0 1.0 0.0 "/Game/Sounds/DefaultSoundAttenuation.DefaultSoundAttenuation" null null null)))

(fn `ToggleEnable`
  (params (enable :type Boolean))
  (bind _buttons (`self.buttons`))
  (bind _display (`self.Display`))
  (bind _output (`|GetArrayItem` _buttons))
  (for _array_element _buttons
    (`/Game/InteractableItems/BP_DiceButton.ToggleEnable` _array_element enable))
  (`TextRenderComponent.K2_SetText` _display "0")
  (`TextRenderComponent.SetTextRenderColor` _display (select `bool` enable :`false` (`/Game/InteractableItems/BP_DiceButton.disabledColor` _output) :`true` (`/Game/InteractableItems/BP_DiceButton.enabledColor` _output)))
  (if enable
    (set `self.prediction` 0)))

(fn `UserConstructionScript`)