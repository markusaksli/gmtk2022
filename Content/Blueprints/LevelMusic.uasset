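; LevelMusic is a Blueprint that drives level music according to the game round and round stage.
; On BeginPlay it picks one of two main loops based on whether the game instance's round is zero, plays it, and binds to the game state's round stage change.
; Dice Roll crossfades from Music to DiceTime, while Round End fades out the audio of every AmbientSound actor in the world.
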(event `self.ReceiveBeginPlay`
  (bind _music (`self.Music`))
  (bind _asbp_game_instance (cast `/Game/Blueprints/BP_GameInstance` (`GameplayStatics.GetGameInstance`)))
  (bind _output_get (set `self.gameInstance` _asbp_game_instance))
  (if (== (`/Game/Blueprints/BP_GameInstance.Round` _output_get) 0)
    (`AudioComponent.SetSound` _music "/Game/Sounds/Music/03_Main_Loop_02.03_Main_Loop_02")
    (else
      (`AudioComponent.SetSound` _music "/Game/Sounds/Music/02_Main_Loop_01__version_2_.02_Main_Loop_01__version_2_")))
  (`AudioComponent.Play` _music 0.0)
  (bind _asbp_game_state (cast `/Game/Blueprints/BP_GameState` (`GameplayStatics.GetGameState`)))
  (bind _output_get_2 (set `self.gameState` _asbp_game_state))
  (add `/Game/Blueprints/BP_GameState.RoundStageChange` _output_get_2 (delegate `OnRoundStageChange`)))

(event `OnRoundStageChange`
  (params (newStage :type "/Game/Blueprints/E_RoundStage Enum" :default "NewEnumerator0"))
  (bind _dicetime (`self.DiceTime`))
  (switch `/Game/Blueprints/E_RoundStage` newStage
    (:`NewEnumerator3`
      (`AudioComponent.FadeOut` (`self.Music`) 2.0 0.0 "Linear")
      (`AudioComponent.Play` _dicetime 0.0)
      (`AudioComponent.FadeIn` _dicetime 5.0 1.0 0.0 "Linear"))
    (:`NewEnumerator4`
      (bind _outactors (`GameplayStatics.GetAllActorsOfClass` "/Script/Engine.AmbientSound"))
      (for _array_element _outactors
        (`AudioComponent.FadeOut` (`AmbientSound.AudioComponent` _array_element) 2.0 0.0 "Linear")))))

(fn `UserConstructionScript`)