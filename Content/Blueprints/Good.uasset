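; One-shot overlap trigger that plays the game's good ending and quits.
; On first overlap it fades out the HUD, waits briefly, then disables player movement and interaction.
; A loop over all ambient sounds fades each out; its body also stops the GameState's ticking, plays the ending sound and starts the HUD's ending text.
; Delays in that loop body space the "GOOD END" text and the quit.
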(event `self.ReceiveActorBeginOverlap`
  (params (OtherActor :type "Actor Object Reference"))
  (if (not (`self.bool`))
    (set `self.bool` true)
    (bind _asbp_game_mode (cast `/Game/Blueprints/BP_GameMode` (`GameplayStatics.GetGameMode`)))
    (`/Game/HUD/WBP_HUD.PlayFadeOut` (`/Game/Blueprints/BP_GameMode.WBP_HUDref` _asbp_game_mode))
    (bind _outactors (`GameplayStatics.GetAllActorsOfClass` "/Script/Engine.AmbientSound"))
    (`KismetSystemLibrary.Delay` 1.0)
    (bind _returnvalue (`GameplayStatics.GetActorOfClass` "/Game/Blueprints/BP_FirstPersonCharacter.BP_FirstPersonCharacter_C"))
    (`/Game/Blueprints/BP_FirstPersonCharacter.ToggleInput` _returnvalue true true)
    (for _array_element _outactors
      (`AudioComponent.FadeOut` (`AmbientSound.AudioComponent` _array_element) 2.0 0.0 "Linear")
      (bind _asbp_game_mode_2 (cast `/Game/Blueprints/BP_GameMode` (`GameplayStatics.GetGameMode`)))
      (bind _wbp_hudref (`/Game/Blueprints/BP_GameMode.WBP_HUDref` _asbp_game_mode_2))
      (`Widget.SetVisibility` (`/Game/HUD/WBP_HUD.EndGameTextBox` _wbp_hudref) "Visible")
      (bind _asbp_game_state (cast `/Game/Blueprints/BP_GameState` (`GameplayStatics.GetGameState`)))
      (set `/Game/Blueprints/BP_GameState.ticking` false _asbp_game_state)
      (`/Game/HUD/WBP_HUD.WriteEndingText` _wbp_hudref "You escape the facility with your life, although you feel different" 15.0)
      (`GameplayStatics.PlaySound2D` "/Game/Sounds/Music/08_Good_Ending.08_Good_Ending" 1.0 1.0 0.0 null null)
      (`KismetSystemLibrary.Delay` 6.0)
      (`/Game/HUD/WBP_HUD.WriteEndingText` _wbp_hudref "GOOD END" 7.0)
      (`KismetSystemLibrary.Delay` 8.0)
      (`KismetSystemLibrary.QuitGame` null "Quit"))))

(fn `UserConstructionScript`)