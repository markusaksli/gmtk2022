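; Game state that runs the dice-prediction round loop through Wake Up, Freeroam, Dice Roll and Round End stages.
; Tick drives a one-second clock, and StageDecider advances stages on timeout, handling delays, input locking, fades and audio.
; Round End checks the BP_Dice prediction against the GameInstance roll, then reloads the level or plays an ending and quits based on GameInstance tallies.
; BeginPlay adds bloom dirt and vignette when the player is punished.
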(event `self.ReceiveBeginPlay`
  (`self.Set Variables`)
  (if (`/Game/Blueprints/BP_GameInstance.Punish` (`self.gameInstance`))
    (bind _returnvalue (`GameplayStatics.GetActorOfClass` "/Script/Engine.PostProcessVolume"))
    (setmembers `PostProcessSettings` :`StructRef` (`PostProcessVolume.Settings` _returnvalue) :`SceneFringeIntensity` 1.36 :`BloomDirtMask` "/Game/Megascans/Surfaces/Dirty_Corrugated_Metal_Sheet_vb1megjew/T_DirtyCorrugatedMetalSheet_vb1megjew_1K_ORDp.T_DirtyCorrugatedMetalSheet_vb1megjew_1K_ORDp" :`BloomDirtMaskIntensity` 1.0 :`BloomDirtMaskTint` (struct :`R` 1.0 :`G` 1.0 :`B` 1.0 :`A` 1.0) :`VignetteIntensity` 0.8)))

(event `self.ReceiveTick`
  (params (DeltaSeconds :type "Float (single-precision)"))
  (if (`self.isChangingState`)
    _
    (elif (> (`self.maxTime`) 0)
      (`self.ClockTick` DeltaSeconds)
      (if (== (`self.seconds`) (`self.maxTime`))
        (set `self.ticking` false)
        (`self.StageDecider` :!label _label))
      (else
        (goto _label)))))

(fn `Check Is Guess Correct`
  (returns (CorrectGuess :type Boolean))
  (bind _diceroll (`/Game/Blueprints/BP_GameInstance.GetDiceRoll` (`self.gameInstance`)))
  (bind _returnvalue (`GameplayStatics.GetActorOfClass` "/Game/Blueprints/BP_Dice.BP_Dice_C"))
  (bind _prediction (`/Game/Blueprints/BP_Dice.prediction` _returnvalue))
  (`KismetSystemLibrary.PrintText` (`|FormatText` "guess: {guess}, dice: {dice}" _prediction _diceroll))
  (bind _display (`/Game/Blueprints/BP_Dice.Display` _returnvalue))
  (`TextRenderComponent.K2_SetText` _display (`KismetTextLibrary.Conv_IntToText` _diceroll))
  (bind _returnvalue_2 (== _prediction _diceroll))
  (`TextRenderComponent.SetTextRenderColor` _display (select `bool` _returnvalue_2 :`false` (make `Color` 0 0 255 255) :`true` (make `Color` 0 255 0 255)))
  (return _returnvalue_2))

(fn `ClockTick`
  (params (deltaSeconds :type "Float (double-precision)"))
  (if (`self.ticking`)
    (bind _output_get (set `self.secondRef` (+ (`self.secondRef`) deltaSeconds)))
    (if (>= _output_get 1.0)
      (bind _output_get_2 (set `self.seconds` (+ 1 (`self.seconds`))))
      (`/Game/Blueprints/BP_ClockComponent.Tick` (`self.BP_ClockComponent`) _output_get_2)
      (set `self.secondRef` 0.0))))

(fn `Set Stage Clock Max Time`
  (params (maxTime :type Integer))
  (bind _output_get (set `self.maxTime` maxTime))
  (set `self.ticking` (> _output_get 0))
  (set `self.seconds` 0))

(fn `TogglePlayerInput`
  (params (Disable :type Boolean))
  (bind _asbp_first_person_character (cast `/Game/Blueprints/BP_FirstPersonCharacter` (`GameplayStatics.GetPlayerCharacter` 0)))
  (`/Game/Blueprints/BP_FirstPersonCharacter.ToggleInput` _asbp_first_person_character Disable Disable))

(fn `UpdateRoundStage`
  (params (NewParam :type "/Game/Blueprints/E_RoundStage Enum" :default "NewEnumerator0"))
  (bind _output_get (set `self.roundStage` NewParam))
  (`self.RoundStageChange` _output_get)
  (`KismetSystemLibrary.PrintString` (`KismetStringLibrary.Concat_StrStr` "Round progressed to " (`|GetEnumeratorNameAsString` _output_get))))

(fn `UserConstructionScript`)